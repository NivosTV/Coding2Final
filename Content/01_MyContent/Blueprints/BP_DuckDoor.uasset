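; BP_DuckDoor is a jail door that opens only for a first-person player who has a key and is flagged IsDuck.
; Overlapping its box checks TotalKeys and IsDuck, printing a "No Keys" or "No friend" message when either check fails.
; On success, a DoOnce spends one key and plays the DoorOpen timeline, which lerps the door mesh downward out of the way.
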(event OnComponentBeginOverlap(Box)
  (params (OverlappedComponent :type Primitive%20Component%20Object%20Reference) (OtherActor :type Actor%20Object%20Reference) (OtherComp :type Primitive%20Component%20Object%20Reference) (OtherBodyIndex :type Integer) (bFromSweep :type Boolean) (SweepResult :type Hit%20Result%20Structure%20%28by%20ref%29))
  (bind _asbp_first_person_character (Utilities|Casting|CastToBP_FirstPersonCharacter OtherActor))
  (if (> (Variables|/Game/01_MyContent/Player/BP_FirstPersonCharacter.BP_FirstPersonCharacter_C|GetTotalKeys _asbp_first_person_character) 0)
    (if (Variables|/Game/01_MyContent/Player/BP_FirstPersonCharacter.BP_FirstPersonCharacter_C|GetIsDuck? _asbp_first_person_character)
      (Utilities|FlowControl|DoOnce false
        (:Completed
          (Math|Integer|DecrementInt (Variables|/Game/01_MyContent/Player/BP_FirstPersonCharacter.BP_FirstPersonCharacter_C|GetTotalKeys _asbp_first_person_character)
            (:%20%20
              (bind _door_open (Timeline|Door%20Open Play)
                (:Update
                  (Transformation|SetRelativeLocation (Variables|Default|GetSM_JailDoor) (Math|Vector|MakeVector 0.0 0.0 (Math|Float|Lerp 0.0 -5e+02 _door_open)) false false)))))))
      (else
        (Development|PrintString "No friend")))
    (else
      (Development|PrintString "No Keys"))))

(fn ConstructionScript)