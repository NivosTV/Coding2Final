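; BP_HealthPotion is an interactable potion actor that the player can pick up, drop or consume to heal.
; PickUp snaps it to the character's Item component, and Drop detaches the bottle mesh if a downward trace hits.
; UsePrimary calls HealPlayer on the first-person character, then destroys the actor.
; Physics and collision toggling, including delayed settling after a drop, sits in disconnected nodes that never run.
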(event EventDrop
  (bind (_outhit _returnvalue) (Collision|LineTraceByChannel (Transformation|GetActorLocation) (- (Transformation|GetActorLocation) "0.000000,0.000000,500.000000") "TraceTypeQuery1" false 0 "None" true "(R=1.000000,G=0.243585,B=0.000000,A=1.000000)" "(R=0.000000,G=1.000000,B=0.622249,A=1.000000)"))
  (if _returnvalue
    (Transformation|DetachFromComponent (Variables|Default|GetSM_Bottle) "KeepWorld" "KeepWorld" "KeepWorld" true)))

(event EventPickUp
  (params (Character :type BP%20First%20Person%20Character%20Object%20Reference))
  (Transformation|AttachComponentToComponent (Variables|/Game/01_MyContent/Player/BP_FirstPersonCharacter.BP_FirstPersonCharacter_C|GetItem Character) "None" "SnapToTarget" "KeepRelative" "KeepRelative" false))

(event EventUsePrimary
  (bind _asbp_first_person_character_1 (Utilities|Casting|CastToBP_FirstPersonCharacter (Game|GetPlayerCharacter 0)))
  (Default|HealPlayer _asbp_first_person_character_1 1e+01)
  (Actor|DestroyActor))

(fn ConstructionScript)