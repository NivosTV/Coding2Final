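; BP_Throwable is an interaction actor that can be picked up and makes noise on impact.
; PickUp attaches it to the character's Item component; nodes that disable mesh physics and collision are present but unconnected.
; Its first hit against anything except the player plays a rock impact sound and reports a short-range noise event instigated by the player, guarded by a DoOnce.
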(event EventPickUp
  (params (Character :type BP%20First%20Person%20Character%20Object%20Reference))
  (Transformation|AttachComponentToComponent (Variables|/Game/01_MyContent/Player/BP_FirstPersonCharacter.BP_FirstPersonCharacter_C|GetItem Character) "None" "SnapToTarget" "KeepRelative" "KeepRelative" false))

(event Collision|EventHit
  (params (MyComp :type Primitive%20Component%20Object%20Reference) (Other :type Actor%20Object%20Reference) (OtherComp :type Primitive%20Component%20Object%20Reference) (bSelfMoved :type Boolean) (HitLocation :type Vector :default "0, 0, 0") (HitNormal :type Vector :default "0, 0, 0") (NormalImpulse :type Vector :default "0, 0, 0") (Hit :type Hit%20Result%20Structure%20%28by%20ref%29))
  (bind _returnvalue (Game|GetPlayerCharacter 0))
  (bind _returnvalue_2 (Transformation|GetActorLocation))
  (if (!= Other _returnvalue)
    (Utilities|FlowControl|DoOnce false
      (:Completed
        (Audio|PlaySoundatLocation "/Game/01_MyContent/Sounds/RockImpact.RockImpact" _returnvalue_2 "0, 0, 0" 1.0 1.0 0.0 0 0 0 0)
        (Class|AISenseHearing|ReportNoiseEvent _returnvalue_2 1.0 _returnvalue 1.5e+02 "None")))))

(fn ConstructionScript)