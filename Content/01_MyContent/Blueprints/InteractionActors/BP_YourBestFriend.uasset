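; BP_YourBestFriend is an interaction actor, a clingy companion that can be picked up, dropped and used to play a quack.
; PickUp snaps it to the character's Item component, and Drop detaches the SMBottle mesh if a downward trace hits.
; Three distance overlap components print pleas as the player leaves, and the first also greets on any overlap.
; Physics-based pickup and drop logic remains in the graph but is disconnected.
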(event OnComponentEndOverlap(Dist_1)
  (params (OverlappedComponent :type Primitive%20Component%20Object%20Reference) (OtherActor :type Actor%20Object%20Reference) (OtherComp :type Primitive%20Component%20Object%20Reference) (OtherBodyIndex :type Integer))
  (Utilities|Casting|CastToBP_FirstPersonCharacter OtherActor)
  (Development|PrintText "Don't leave your best friend!"))

(event OnComponentEndOverlap(Dist_2)
  (params (OverlappedComponent :type Primitive%20Component%20Object%20Reference) (OtherActor :type Actor%20Object%20Reference) (OtherComp :type Primitive%20Component%20Object%20Reference) (OtherBodyIndex :type Integer))
  (Utilities|Casting|CastToBP_FirstPersonCharacter OtherActor)
  (Development|PrintText "Why are you leaving  me?"))

(event OnComponentEndOverlap(Dist_3)
  (params (OverlappedComponent :type Primitive%20Component%20Object%20Reference) (OtherActor :type Actor%20Object%20Reference) (OtherComp :type Primitive%20Component%20Object%20Reference) (OtherBodyIndex :type Integer))
  (Utilities|Casting|CastToBP_FirstPersonCharacter OtherActor)
  (Development|PrintText "DONT LEAVE ME, PLEASE GOD DONT LEAVE"))

(event OnComponentBeginOverlap(Dist_1)
  (params (OverlappedComponent :type Primitive%20Component%20Object%20Reference) (OtherActor :type Actor%20Object%20Reference) (OtherComp :type Primitive%20Component%20Object%20Reference) (OtherBodyIndex :type Integer) (bFromSweep :type Boolean) (SweepResult :type Hit%20Result%20Structure%20%28by%20ref%29))
  (Development|PrintText "Hello!"))

(event EventDrop
  (bind (_outhit _returnvalue) (Collision|LineTraceByChannel (Transformation|GetActorLocation) (- (Transformation|GetActorLocation) "0.000000,0.000000,500.000000") "TraceTypeQuery1" false 0 "None" true "(R=1.000000,G=0.243585,B=0.000000,A=1.000000)" "(R=0.000000,G=1.000000,B=0.622249,A=1.000000)"))
  (if _returnvalue
    (Transformation|DetachFromComponent (Variables|Default|GetSM_Bottle) "KeepWorld" "KeepWorld" "KeepWorld" true)))

(event EventPickUp
  (params (Character :type BP%20First%20Person%20Character%20Object%20Reference))
  (Transformation|AttachComponentToComponent (Variables|/Game/01_MyContent/Player/BP_FirstPersonCharacter.BP_FirstPersonCharacter_C|GetItem Character) "None" "SnapToTarget" "KeepRelative" "KeepRelative" false))

(event EventUsePrimary
  (Audio|PlaySound2D "/Game/01_MyContent/Sounds/Quack.Quack" 1.0 1.0 0.0 0 0))

(fn ConstructionScript)